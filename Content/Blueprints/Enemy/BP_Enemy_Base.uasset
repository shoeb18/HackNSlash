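; Base enemy Blueprint that handles the dissolve effect when the enemy dies.
; OnEnemyDied pauses mesh animation, disables capsule collision and async loads the supplied Niagara system.
; Once loaded, it attaches the system to the mesh, tinting particles with the material's dissolve edge color.
; A timeline scaled by TotalDissolveTime then drives the mesh's DissolveAmount parameter and destroys the actor when finished.
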(event `self.ReceiveBeginPlay`)

(event `/Game/Blueprints/Enemy/BPI_EnemyDeath.OnEnemyDied`
  (params (DissolveNiagaraSystem :type "NiagaraSystem Soft Object Reference"))
  (bind _mesh (`self.Mesh`))
  (`|ExecutionSequence`
    (:`then_0`
      (set `SkeletalMeshComponent.bPauseAnims` true (`self.Mesh`))
      (`PrimitiveComponent.SetCollisionEnabled` (`self.CapsuleComponent`) "NoCollision"))
    (:`then_1`
      (bind _object (`|LoadAsset` DissolveNiagaraSystem)
        (:`Completed`
          (bind _asniagara_system (cast `NiagaraSystem` _object))
          (bind _returnvalue (`NiagaraFunctionLibrary.SpawnSystemAttached` _asniagara_system (`self.Mesh`) "None" (0.0 0.0 0.0) (struct) "KeepRelativeOffset" true))
          (bind _returnvalue_2 (`PrimitiveComponent.CreateDynamicMaterialInstance` _mesh 0 (`PrimitiveComponent.GetMaterial` _mesh 0) "None"))
          (bind _returnvalue_3 (`MaterialInstanceDynamic.K2_GetVectorParameterValue` _returnvalue_2 "DissolveEdgeColor"))
          (`NiagaraComponent.SetNiagaraVariableLinearColor` _returnvalue "DissolveParticleColor" _returnvalue_3)
          (`TimelineComponent.SetPlayRate` (`self.Dissolve Timeline`) (/ 1.0 (`self.TotalDissolveTime`)))
          (bind (_direction _normalizedfloat) (`Timeline|Dissolve Timeline` :!via `PlayFromStart`)
            (:`Update`
              (`MeshComponent.SetScalarParameterValueOnMaterials` (`self.Mesh`) "DissolveAmount" _normalizedfloat))
            (:`Finished`
              (`self.K2_DestroyActor`))))))))

(fn `UserConstructionScript`)