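; Player hero Blueprint that prototypes camera transitions, with debug prints of camera-to-actor alignment.
; Shift sprints and eases the camera to a shoulder mount by reattaching it and using MoveComponentTo.
; TriggerActionCam uses the same technique, first flipping the action spring arm by the sign of the camera-forward/actor-right dot product.
; FlipFlop-driven timelines toggle post-process changes through CameraExposure and a test spring-arm move on T.
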(event `self.ReceiveTick`
  (params (DeltaSeconds :type "Float (single-precision)"))
  (`KismetSystemLibrary.PrintString` (`KismetStringLibrary.Concat_StrStr` "Forward : " (`KismetStringLibrary.Conv_DoubleToString` (`KismetMathLibrary.Dot_VectorVector` (`self.GetActorForwardVector`) (`SceneComponent.GetForwardVector` (`self.CameraComponent`))))) true true (struct :`G` 0.630208 :`B` 0.025551 :`A` 1.0) 2.0 "1")
  (`KismetSystemLibrary.PrintString` (`KismetStringLibrary.Concat_StrStr` "Right : " (`KismetStringLibrary.Conv_DoubleToString` (`KismetMathLibrary.Dot_VectorVector` (`self.GetActorRightVector`) (`SceneComponent.GetForwardVector` (`self.CameraComponent`))))) true true (struct :`R` 1.0 :`B` 0.021375 :`A` 1.0) 2.0 "2"))

(event `Key|LeftShift`
  (params (Key :type "Key Structure"))
  (bind _charactermovement (`self.CharacterMovement`))
  ; Test Sprint
  (:`Pressed`
    (set `CharacterMovementComponent.MaxWalkSpeed` 1000.0 _charactermovement)
    (`SceneComponent.K2_AttachToComponent` (`self.CameraComponent`) (`self.Test_ShouldCam`) "None" "KeepWorld" "KeepWorld" "KeepWorld" true)
    (`KismetSystemLibrary.MoveComponentTo` (`self.CameraComponent`) (0.0 0.0 0.0) (struct) true true 1.0 true))
  (:`Released`
    (set `CharacterMovementComponent.MaxWalkSpeed` 500.0 _charactermovement)
    (`SceneComponent.K2_AttachToComponent` (`self.CameraComponent`) (`self.SpringArmComponent`) "None" "KeepWorld" "KeepWorld" "KeepWorld" true)
    (`KismetSystemLibrary.MoveComponentTo` (`self.CameraComponent`) (0.0 0.0 0.0) (struct) true true 0.5 true)))

(event `Trigger Action Cam`
  (params (`Trigger Action Cam` :type Boolean) (`Attachment Rules` :type "EAttachmentRule Enum" :default "KeepRelative"))
  ; Trigger Action Cam
  (`self.SetSpringArmRotation`)
  (if `Trigger Action Cam`
    (`SceneComponent.K2_AttachToComponent` (`self.CameraComponent`) (`self.ActionCam_SpringArm`) "None" `Attachment Rules` `Attachment Rules` `Attachment Rules` true)
    (`KismetSystemLibrary.MoveComponentTo` (`self.CameraComponent`) (0.0 0.0 0.0) (struct) true true 0.3 true)
    (else
      (`SceneComponent.K2_AttachToComponent` (`self.CameraComponent`) (`self.SpringArmComponent`) "None" "KeepWorld" "KeepWorld" "KeepWorld" true)
      (`KismetSystemLibrary.MoveComponentTo` (`self.CameraComponent`) (0.0 0.0 0.0) (struct) true true 0.6 true))))

(event `CameraExposure`
  (`/Engine/EditorBlueprintResources/StandardMacros.FlipFlop`
    (:`A`
      (bind (_direction _newtrack_0) (`Timeline|Timeline_0` :!label _label)
        (:`Update`
          (set `CameraComponent.PostProcessSettings` (make `PostProcessSettings` :`AutoExposureBias` _newtrack_0) (`self.CameraComponent`)))))
    (:`B`
      (goto _label :!via `Reverse`))))

(event `Key|T`
  (params (Key :type "Key Structure"))
  (bind _springarmcomponent (`self.SpringArmComponent`))
  ; Action Cam Test In Timeliine
  (:`Pressed`
    (set `SpringArmComponent.bUsePawnControlRotation` false (`self.SpringArmComponent`))
    (`/Engine/EditorBlueprintResources/StandardMacros.FlipFlop`
      (:`A`
        (bind (_direction _alpha _location) (`Timeline|Timeline` :`NewTime` 0.5 :!label _label_2)
          (:`Update`
            (`SceneComponent.K2_SetRelativeLocationAndRotation` (`self.SpringArmComponent`) (`KismetMathLibrary.MakeVector` (.x _location)) (`KismetMathLibrary.MakeRotator` 0.0 0.0 _alpha) false false))
          (:`Finished`
            (set `SpringArmComponent.bUsePawnControlRotation` true _springarmcomponent)
            (`Controller.SetControlRotation` (`self.GetController`) (`SceneComponent.K2_GetComponentRotation` _springarmcomponent)))))
      (:`B`
        (goto _label_2 :!via `Reverse`)))))

(fn `SetSpringArmRotation`
  (if (< (`KismetMathLibrary.Dot_VectorVector` (`self.GetActorRightVector`) (`SceneComponent.GetForwardVector` (`self.CameraComponent`))) 0.0)
    (`SceneComponent.K2_SetRelativeRotation` :`self` (`self.ActionCam_SpringArm`))
    (`KismetSystemLibrary.PrintString` "Move Spring Arm to the Right")
    (else
      (`SceneComponent.K2_SetRelativeRotation` (`self.ActionCam_SpringArm`) (struct :`Yaw` 180.0) false false)
      (`KismetSystemLibrary.PrintString` "Move Spring Arm to the Left"))))

(fn `UserConstructionScript`)